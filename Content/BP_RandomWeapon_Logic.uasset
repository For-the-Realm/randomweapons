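; Mordhau actor that swaps a player's equipment for random weapons whenever they control a new character, such as after respawning.
; Each Tick it casts its attach parent to the player controller and compares the controlled character with the cached LastCharacter.
; On a change, it loops over Equipment, dropping and destroying each item, then spawning a random weapon, randomizing its customization and making the character pick it up.
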(event `self.ReceiveBeginPlay`)

(event `self.ReceiveTick`
  (params (DeltaSeconds :type "Float (single-precision)"))
  (bind _last_character (`self.Last Character`))
  ;[1 1 1] Check if character has changed from the last time we saved it. This would imply that a Character has died and respawned.
  (bind _returnvalue (`MordhauUtilityLibrary.GetAttachParentActor` self))
  (bind _asbp_mordhau_player_controller (cast `/Game/Mordhau/Blueprints/BP_MordhauPlayerController` _returnvalue))
  (bind _returnvalue_2 (`MordhauPlayerController.GetControlledMordhauCharacter` _asbp_mordhau_player_controller true))
  (if (!= (`self.Last Character`) _returnvalue_2)
    (set `self.Last Character` _returnvalue_2)
    (for _array_element (`MordhauCharacter.Equipment` _last_character)
      (bind _returnvalue_3 (`MordhauCharacter.DropEquipment` _last_character _array_element false))
      (`self.K2_DestroyActor` _returnvalue_3)
      (bind (_id _returnvalue_4) (`MordhauUtilityLibrary.GetRandomWeapon` (make `SkillsCustomization`) "Exclusive"))
      (bind _returnvalue_5 (`|SpawnActorFromClass` (`GameplayStatics.GetObjectClass` _returnvalue_4) (`KismetMathLibrary.MakeTransform` (0.0 0.0 0.0)) "AlwaysSpawn" "OverrideRootScale" null null))
      (bind _returnvalue_6 (`MordhauEquipment.GetRandomCustomization` _returnvalue_5 false))
      (`MordhauEquipment.AssignCustomization` _returnvalue_5 _returnvalue_6 0 0 0)
      (`MordhauCharacter.PickUp` (`self.Last Character`) _returnvalue_5 -1))))

(fn `UserConstructionScript`)